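; Game mode that serves as a MySQL access point, wrapping a BPMySQLComponent.
; DoConnectDB stores the schema, prints the connection arguments including the password, binds a connected event and starts the connection.
; EventDBConnected applies the stored schema.
; DoInsertDB and DoSelectDB pass a table name, username and password to the component and return its result.
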(event EventBeginPlay)

(event EventTick
  (params (DeltaSeconds :type Float%20%28single-precision%29)))

(fn ConstructionScript)

(fn DoConnectDB
  (params (host :type String) (port :type Integer) (username :type String) (password :type String) (schema :type String))
  (bind _bp_mysqlcomponent (Variables|Default|GetBP_MySQLComponent))
  (Variables|Default|SetSchema schema)
  (Development|PrintString (Utilities|String|Append "DoConnectDB[" host "," (Utilities|String|ToString(Integer) port) "," username "," password "," schema "]") true true "(R=0.000000,G=0.660000,B=1.000000,A=1.000000)" 5.0)
  (EventDispatchers|BindEventtoEventDBConnected _bp_mysqlcomponent (EventDispatchers|CreateEvent :!event EventDBConnected))
  (bind _returnvalue (Class|MySQLComponent|ConnecttoDatabase _bp_mysqlcomponent host port username password))
  (return _returnvalue))

(fn DoInsertDB
  (params (tablename :type String) (username :type String) (password :type String))
  (bind _returnvalue (Class|MySQLComponent|InsertIntoDatabase (Variables|Default|GetBP_MySQLComponent) tablename username password))
  (return _returnvalue))

(fn DoSelectDB
  (params (tablename :type String) (username :type String) (password :type String))
  (bind _returnvalue (Class|MySQLComponent|SelectfromDatabase (Variables|Default|GetBP_MySQLComponent) tablename username password))
  (return _returnvalue))

(fn EventDBConnected
  (Class|MySQLComponent|UseSchema (Variables|Default|GetBP_MySQLComponent) (Variables|Default|GetSchema)))